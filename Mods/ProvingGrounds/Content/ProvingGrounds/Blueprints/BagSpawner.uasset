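; BagSpawner is an unfinished Proving Grounds Blueprint that, despite its name, spawns nothing and has an empty construction script.
; A disconnected test chain queries the Asset Registry for SBZBagType assets and synchronously loads the first few through soft object paths.
; It casts each to SBZBagType and prints whether that worked, but nothing triggers this chain, so it never runs.
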(fn ConstructionScript)