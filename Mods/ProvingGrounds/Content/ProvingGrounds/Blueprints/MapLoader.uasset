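; Proving Grounds actor that swaps between the Proving Grounds and PAYDAY 3 maps at runtime.
; UnloadMap freezes players, clears AI visibility lists to avoid a crash, then removes current levels and non-baseline actors.
; LoadMap streams in folder levels found via the Asset Registry as sequential instances, skipping R_/M_ names.
; It then optionally strips guards, AI, objectives and security, resets doors, and retries until a player start exists for teleporting.
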(event Custom|UnloadMap
  (params (MapIDX :type Integer) (ReturnToPG :type Boolean) (RemoveCoding :type Boolean))
  (bind _returnvalue (Class|SBZAIVisibilityManager|GetAIVisibilityManager))
  ;[1 1 1] Stale AI Visibility Actors cause a crash in ASBZAIVisibilityManager::OnDynVisibilityUpdated
  (Utilities|Array|Clear (Variables|/Script/Starbreeze.SBZAIVisibilityManager|GetAIVisibilityRelevantActorsAutomatic _returnvalue))
  (Utilities|Array|Clear (Variables|/Script/Starbreeze.SBZAIVisibilityManager|GetAIVisibilityRelevantActorsEveryFrame _returnvalue))
  (Utilities|Array|Clear (Variables|/Script/Starbreeze.SBZAIVisibilityManager|GetAIVisibilityRelevantActorsToRefreshAfterUpdate _returnvalue))
  (Utilities|Map|Clear (Variables|/Script/Starbreeze.SBZAIVisibilityManager|GetAIVisibilityRelevants _returnvalue))
  (Class|SBZAIVisibilityManager|UnregisterVisibilityComponent _returnvalue (Variables|/Script/Starbreeze.SBZAIVisibilityManager|GetVisibilityComponent _returnvalue))
  (Variables|Default|SetRemoveCodingSwitch RemoveCoding)
  (CallFunction|PrinttoModLoader (Utilities|String|Append "message gotten idx is " (Utilities|String|ToString(Integer) MapIDX)))
  (CallFunction|DisableCharacterMovement true)
  (if (Variables|Default|GetAtPG)
    (Class|GameplayStatics|UnloadStreamLevelbySoftObjectPtr "/ProvingGrounds/ProvingGrounds/ProvingGroundLighting.ProvingGroundLighting" false)
    (Class|GameplayStatics|UnloadStreamLevelbySoftObjectPtr "/ProvingGrounds/ProvingGrounds/PGEnviroment.PGEnviroment" false)
    (Variables|Default|SetAtPG false)
    (bind _outactors (Actor|GetAllActorsOfClass "/Script/Engine.Actor"))
    (bind _output_get (Variables|Default|SetBaseActors _outactors))
    (bind _returnvalue_2 (Actor|GetActorOfClass "/Script/Engine.PlayerStart"))
    (Variables|Default|SetSpawnLocation _returnvalue_2)
    (else
      (for _array_element (Variables|Default|GetLoadedMaps)
        (Class|LevelStreaming|SetIsRequestingUnloadandRemoval _array_element true))
      (bind _outactors_2 (Actor|GetAllActorsOfClass "/Script/Engine.Actor"))
      (for _array_element_2 _outactors_2
        (if (not (Utilities|Array|ContainsItem _output_get _array_element_2))
          (Actor|DestroyActor _array_element_2)
          (bind _aspd3heist_game_state (Utilities|Casting|CastToPD3HeistGameState (Game|GetGameState)))
          (Variables|/Script/Starbreeze.PD3HeistGameState|SetAnswerPagerCount _aspd3heist_game_state 0)))
      (Utilities|Array|Clear (Variables|Default|GetLoadedMaps))))
  (CallFunction|LoadMap MapIDX ReturnToPG))

(event Custom|LoadMap
  (params (MapIDX :type Integer) (ReturnToPG :type Boolean))
  (bind _outassetdata (Class|AssetRegistry|GetAssetsbyPath (Class|AssetRegistryHelpers|GetAssetRegistry) (Utilities|String|StringToName (.LeftS (Utilities|String|Split (Utilities|BreakSoftObjectPath (Class|SBZOnlineFunctionLibrary|GetPathNamefromLevelIdx MapIDX)) "/" "IgnoreCase" "FromEnd"))) true false))
  (Variables|Default|SetADS _outassetdata)
  (CallFunction|LoadLoop ReturnToPG))

(event Custom|LoadLoop
  (params (ReturnToPG :type Boolean))
  (bind _ads (Variables|Default|GetADS))
  (bind _loadingindex (Variables|Default|GetLoadingIndex))
  (bind _output (Utilities|Array|Get(acopy) _ads _loadingindex))
  (bind _assetname (Utilities|Struct|BreakAssetData _output))
  (if ReturnToPG
    (Class|GameplayStatics|LoadStreamLevelbySoftObjectPtr "/ProvingGrounds/ProvingGrounds/PGEnviroment.PGEnviroment" true false)
    (Class|GameplayStatics|LoadStreamLevelbySoftObjectPtr "/ProvingGrounds/ProvingGrounds/ProvingGroundLighting.ProvingGroundLighting" true false)
    (Utilities|FlowControl|Delay 0.5)
    (if (Variables|Default|GetRemoveCodingSwitch) :!label _label
      _
      (elif ReturnToPG
        _
        (else
          (CallFunction|RemoveCoding))))
    (CallFunction|TeleportEvent ReturnToPG)
    (elif (< _loadingindex (Utilities|Array|Length _ads))
      (if (or (Utilities|String|StartsWith (Utilities|String|ToString(Name) _assetname) "R_" "CaseSensitive") (Utilities|String|StartsWith (Utilities|String|ToString(Name) _assetname) "M_" "CaseSensitive"))
        (Utilities|Array|Add (Variables|Default|GetLoadedMaps) (stale _returnvalue) :!label _label_2)
        (Math|Integer|IncrementInt (Variables|Default|GetLoadingIndex)
          (:%20%20
            (CallFunction|LoadLoop ReturnToPG)))
        (else
          (bind _returnvalue (Class|LevelStreamingDynamic|LoadLevelInstance (Utilities|String|ToString(Name) _assetname) "0, 0, 0" "0, 0, 0" (Utilities|String|ToString(Name) _assetname) 0 false))
          (Utilities|FlowControl|Delay 0.05)
          (bind _output_get (Variables|Default|SetTempLevelVar _returnvalue))
          (Utilities|FlowControl|ForLoopwithBreak 0 100 :!label _label_3
            (:LoopBody
              (if (Class|LevelStreaming|IsLevelLoaded _output_get)
                (goto _label_3 Break)
                (else
                  (Utilities|FlowControl|Delay 0.05))))
            (:Completed
              (CallFunction|PrinttoModLoader (Utilities|String|Append "Map name " (Utilities|String|ToString(Name) _assetname)))
              (goto _label_2)))))
      (else
        (goto _label)))))

(event Custom|WaitUntilLoaded
  (Utilities|FlowControl|ForLoopwithBreak 0 100 :!label _label
    (:LoopBody
      (if (Class|LevelStreaming|IsLevelLoaded (stale Custom|LoadLoop _output_get))
        (goto _label Break)
        (else
          (Utilities|FlowControl|Delay 0.05))))
    (:Completed
      (CallFunction|PrinttoModLoader (Utilities|String|Append "Map name " (Utilities|String|ToString(Name) (.AssetName (Utilities|Struct|BreakAssetData (Utilities|Array|Get(acopy) (Variables|Default|GetADS) (Variables|Default|GetLoadingIndex)))))))
      (Utilities|Array|Add (Variables|Default|GetLoadedMaps) (stale Custom|LoadLoop _returnvalue))
      (Math|Integer|IncrementInt (Variables|Default|GetLoadingIndex)
        (:%20%20
          (CallFunction|LoadLoop (stale Custom|LoadLoop ReturnToPG)))))))

(event Custom|TeleportEvent
  (params (ReturnToPG :type Boolean))
  (Variables|Default|SetLoadingIndex 0)
  (Variables|Default|SetAtPG ReturnToPG)
  (bind _returnvalue (Actor|GetActorOfClass "/Script/Starbreeze.SBZPlayerStartGroup"))
  (if (Utilities|IsValid _returnvalue)
    (CallFunction|PrinttoModLoader)
    (CallFunction|PrinttoModLoader (Utilities|String|Append (Utilities|String|ToString(Vector) (Transformation|GetActorLocation (Utilities|Array|Get(acopy) (Variables|/Script/Starbreeze.SBZPlayerStartGroup|GetPlayerStarts _returnvalue)))) " spawn location"))
    (CallFunction|TeleportPlayers (Transformation|GetActorLocation (Utilities|Array|Get(acopy) (Variables|/Script/Starbreeze.SBZPlayerStartGroup|GetPlayerStarts _returnvalue))) (Transformation|GetActorRotation (Utilities|Array|Get(acopy) (Variables|/Script/Starbreeze.SBZPlayerStartGroup|GetPlayerStarts _returnvalue))))
    (Utilities|FlowControl|Delay 0.5)
    (CallFunction|DisableCharacterMovement false)
    (else
      (Utilities|FlowControl|Delay 0.25)
      (CallFunction|RetrySpawnSearch))))

(event Custom|RemoveCoding
  (Utilities|FlowControl|Sequence
    (:then_1
      (bind _outactors (Actor|GetAllActorsOfClass "/Game/Gameplay/Characters/Cop/CH_SecurityGuard.CH_SecurityGuard_C"))
      (for _array_element _outactors
        (Actor|DestroyActor _array_element)
        (bind _aspd3heist_game_state (Utilities|Casting|CastToPD3HeistGameState (Game|GetGameState)))
        (Variables|/Script/Starbreeze.PD3HeistGameState|SetAnswerPagerCount _aspd3heist_game_state 0)))
    (:then_2
      (bind _outactors_2 (Actor|GetAllActorsOfClass "/Script/Starbreeze.SBZAICharacter"))
      (for _array_element_2 _outactors_2
        (Actor|DestroyActor _array_element_2)))
    (:then_3
      (bind _outactors_3 (Actor|GetAllActorsOfClass "/Script/Starbreeze.SBZPlayerTriggerVolume"))
      (for _array_element_3 _outactors_3
        (Actor|DestroyActor _array_element_3)))
    (:then_4
      (bind _foundwidgets (Widget|GetAllWidgetsOfClass "/Script/Starbreeze.SBZObjectiveWidget" false))
      (for _array_element_4 _foundwidgets
        (for _array_element_5 (Class|PanelWidget|GetAllChildren (Variables|/Script/Starbreeze.SBZObjectiveWidget|GetPanel_SubObjectivesContainer _array_element_4))
          (Widget|RemovefromParent _array_element_5))))
    (:then_5
      (bind _outactors_4 (Actor|GetAllActorsOfClass "/Script/Starbreeze.SBZObjective"))
      (for _array_element_6 _outactors_4
        (Actor|DestroyActor _array_element_6)))
    (:then_6
      (bind _outactors_5 (Actor|GetAllActorsOfClass "/Game/Gameplay/Props/BP_SecurityCamera.BP_SecurityCamera_C"))
      (for _array_element_7 _outactors_5
        (Actor|DestroyActor _array_element_7)))
    (:then_7
      (bind _outactors_6 (Actor|GetAllActorsOfClass "/Script/Starbreeze.SBZInteractableDoor"))
      (for _array_element_8 _outactors_6
        (Variables|/Script/Starbreeze.SBZGate|SetServerState _array_element_8 "Closed")
        (Class|SBZGate|SetState _array_element_8 "Closed")
        (Variables|/Script/Starbreeze.SBZGate|SetInitialState _array_element_8 "Closed")
        (Class|SBZInteractableComponent|SetInteractionEnabled (Variables|/Script/Starbreeze.SBZInteractableGate|GetInteractable _array_element_8) true)))
    (:then_8
      (bind _outactors_7 (Actor|GetAllActorsOfClass "/Script/Starbreeze.SBZPawnSpawnPredefined"))
      (for _array_element_9 _outactors_7
        (Actor|DestroyActor _array_element_9)))
    (:then_9
      (bind _outactors_8 (Actor|GetAllActorsOfClass "/Script/Starbreeze.SBZLaserGrid"))
      (for _array_element_10 _outactors_8
        (Actor|DestroyActor _array_element_10)))
    (:then_10
      (bind _outactors_9 (Actor|GetAllActorsOfClass "/Game/Gameplay/Props/BP_MovingMotionSensor.BP_MovingMotionSensor_C"))
      (for _array_element_11 _outactors_9
        (Actor|DestroyActor _array_element_11)))
    (:then_11
      (bind _outactors_10 (Actor|GetAllActorsOfClass "/Game/Prototype/Blueprints/Bags/BP_BaseValuableBag.BP_BaseValuableBag_C"))
      (for _array_element_12 _outactors_10
        (Actor|DestroyActor _array_element_12))
      (bind _outactors_11 (Actor|GetAllActorsOfClass "/Game/Prototype/Blueprints/Bags/BP_BaseEquipmentBag.BP_BaseEquipmentBag_C"))
      (for _array_element_13 _outactors_11
        (Actor|DestroyActor _array_element_13)))))

(event Custom|RetrySpawnSearch
  (CallFunction|PrinttoModLoader "Spawn not found, retrying!")
  (bind _returnvalue (Actor|GetActorOfClass "/Script/Starbreeze.SBZPlayerStartGroup"))
  (if (Utilities|IsValid _returnvalue)
    (CallFunction|PrinttoModLoader)
    (CallFunction|PrinttoModLoader (Utilities|String|Append (Utilities|String|ToString(Vector) (Transformation|GetActorLocation (Utilities|Array|Get(acopy) (Variables|/Script/Starbreeze.SBZPlayerStartGroup|GetPlayerStarts _returnvalue)))) " spawn location"))
    (CallFunction|TeleportPlayers (Transformation|GetActorLocation (Utilities|Array|Get(acopy) (Variables|/Script/Starbreeze.SBZPlayerStartGroup|GetPlayerStarts _returnvalue))) (Transformation|GetActorRotation (Utilities|Array|Get(acopy) (Variables|/Script/Starbreeze.SBZPlayerStartGroup|GetPlayerStarts _returnvalue))))
    (Utilities|FlowControl|Delay 0.5)
    (CallFunction|DisableCharacterMovement false)
    (else
      (Utilities|FlowControl|Delay 0.25)
      (CallFunction|RetrySpawnSearch))))

(event EventBeginPlay)

(fn ConstructionScript)

(fn DisableCharacterMovement
  (params (Disabled :type Boolean))
  (for _array_element (Class|SBZPlayerLibrary|GetAllSBZPlayerCharacters)
    (if Disabled
      (Pawn|Components|CharacterMovement|SetMovementMode (Variables|/Script/Engine.Character|GetCharacterMovement _array_element) "MOVE_None" 0)
      (else
        (Pawn|Components|CharacterMovement|SetMovementMode (Variables|/Script/Engine.Character|GetCharacterMovement _array_element) "MOVE_Walking" 0)))))

(fn TeleportPlayers
  (params (Location :type Vector) (Rotation :type Rotator))
  (for _array_element (Class|SBZPlayerLibrary|GetAllSBZPlayerCharacters)
    (Transformation|Teleport _array_element Location Rotation)))