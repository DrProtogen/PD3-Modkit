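; InteractionReader is a Proving Grounds display Blueprint that positions a referenced interaction actor and labels it with its identifying information.
; The construction script moves InteractionBP to the InteractionLocation component's world position plus world-space forward (Y) and height (Z) offsets, applying RotationOffset as its absolute rotation.
; On BeginPlay, it fills text elements with that actor's display name, class display name and object path.
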(event EventBeginPlay
  (bind _interactionbp (Variables|Default|GetInteractionBP))
  (Rendering|Components|TextRender|SetText (Variables|Default|GetDisplayName) (Utilities|Text|ToText(String) (Utilities|GetDisplayName _interactionbp)))
  (Rendering|Components|TextRender|SetText (Variables|Default|GetClassName) (Utilities|Text|ToText(String) (Utilities|GetClassDisplayName (Utilities|GetClass _interactionbp))))
  (Rendering|Components|TextRender|SetText (Variables|Default|GetFileLocation) (Utilities|Text|ToText(String) (Class|KismetSystemLibrary|GetPathName _interactionbp))))

(fn ConstructionScript
  (Transformation|SetActorLocationAndRotation (Variables|Default|GetInteractionBP) (+ (Transformation|GetWorldLocation (Variables|Default|GetInteractionLocation)) (Math|Vector|MakeVector 0.0 (Math|Conversions|ToFloat(Integer) (Variables|Default|GetFowardOffset)) (Variables|Default|GetHeightOffset))) (Variables|Default|GetRotationOffset)))