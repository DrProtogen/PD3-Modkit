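; Mod actor that quick-loads the Proving Grounds map as a solo game.
; On Init it scans the level list for a path containing LVL_ProvingGrounds and asks the game state machine to start that level, skipping pre-match.
; ParseHUDData and AddSettingsStackToMenu are empty stubs, with disconnected leftover nodes for versioned HUD settings save games.
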(event EventInit
  (for _index (range 0 (Utilities|Array|Length (Class|SBZGameStateMachineSettings|GetLevels)))
    (if (Utilities|String|Contains (Utilities|BreakSoftObjectPath (Class|SBZOnlineFunctionLibrary|GetPathNamefromLevelIdx 0 _index)) "LVL_ProvingGrounds" true)
      (Class|SBZGameStateMachine|RequestSoloGame (Class|SBZGameStateMachineFunctionLibrary|GetGameStateMachine) _index 0 true))))

(fn ConstructionScript)

(fn ParseHUDData
  (params (DA :type %20Object%20Reference)))

(fn AddSettingsStacktoMenu)