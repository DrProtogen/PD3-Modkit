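; BP_SpawnGroup is a map-unit actor for a spawn group that records which room volume it sits in.
; On BeginPlay it stores the result of GetCurrentRoom in SpawnGroupRoom.
; That function scans every SBZRoomVolume, treating a zero closest-point collision distance as containment and keeping the last match.
; It prints the volume count and found room name to the mod loader; no spawning logic appears here.
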(event EventBeginPlay
  (Variables|Default|SetSpawnGroupRoom (CallFunction|GetCurrentRoom self)))

(fn ConstructionScript)

(fn GetCurrentRoom
  (bind _outactors (Actor|GetAllActorsOfClass self "/Script/Starbreeze.SBZRoomVolume"))
  (CallFunction|PrinttoModLoader (Utilities|String|ToString(Integer) (Utilities|Array|Length _outactors)))
  (bind _array_element (Utilities|Array|ForEachLoopwithBreak _outactors)
    (:LoopBody
      (if (== (.ReturnValue (Collision|GetClosestPointonCollision (Variables|/Script/Engine.Brush|GetBrushComponent _array_element) (Transformation|GetActorLocation) "None")) 0.0)
        (LocalVariables|SetFoundRoom _array_element)))
    (:Completed
      (CallFunction|PrinttoModLoader (Utilities|GetDisplayName (LocalVariables|GetFoundRoom)))
      (return (LocalVariables|GetFoundRoom)))))