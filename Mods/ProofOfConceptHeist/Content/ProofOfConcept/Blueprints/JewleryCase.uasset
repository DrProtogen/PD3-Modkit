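; JewleryCase is a proof-of-concept jewelry case that fills itself with jewelry actors at runtime.
; On BeginPlay it spawns a low-value interactable jewelry actor at its StaticMesh transform and enables that actor's interaction.
; It also spawns a jewelry display actor at the CounterJewelry01Display128 component's transform, offsetting the yaw by a quarter turn.
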(event EventBeginPlay
  (bind _counterjewelry_01_display_128 (Variables|Default|GetCounterJewelry_01_Display_128))
  (bind _returnvalue (Transformation|GetWorldTransform _counterjewelry_01_display_128))
  (bind (_location _rotation _scale) (Math|Transform|BreakTransform _returnvalue))
  (bind (_roll _pitch _yaw) (Math|Rotator|BreakRotator _rotation))
  (bind _returnvalue_2 (Game|SpawnActorfromClass "/Game/Prototype/Blueprints/Bags/BP_InteractableJewelry_LowValue.BP_InteractableJewelry_LowValue_C" (Transformation|GetWorldTransform (Variables|Default|GetStaticMesh)) "Undefined" "MultiplyWithRoot" 0 0))
  (Class|SBZInteractableComponent|SetInteractionEnabled (Variables|/Script/Starbreeze.SBZSingleBagGenerator|GetInteractable _returnvalue_2) true)
  (Game|SpawnActorfromClass "/Game/Prototype/Blueprints/DisplayCases/BP_JewelryDisplay_128.BP_JewelryDisplay_128_C" (Math|Transform|MakeTransform _location (Math|Rotator|MakeRotator _roll _pitch (- _yaw 9e+01)) _scale) "Undefined" "MultiplyWithRoot" 0 0))

(event Collision|EventActorBeginOverlap
  (params (OtherActor :type Actor%20Object%20Reference)))

(event EventTick
  (params (DeltaSeconds :type Float%20%28single-precision%29)))

(fn ConstructionScript)