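; Front gate Blueprint in a proof-of-concept folder that raises its doors when the OpenDoors event fires.
; After a five-second delay, a Timeline drives lerps on the relative locations of three CubeGrid-modeled components, lifting them vertically together.
; Start and end positions are hardcoded, and the graph has no closing logic.
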(event Custom|OpenDoors
  (Utilities|FlowControl|Delay 5.0)
  (bind _newtrack_0 (Timeline|Timeline Play)
    (:Update
      (Transformation|SetRelativeLocation (Variables|Default|GetCubeGridToolOutput_C6FC7465) (Math|Vector|Lerp(Vector) "276.000000,123.375000,0.000000" "276.000000,123.375000,250.000000" _newtrack_0) false false)
      (Transformation|SetRelativeLocation (Variables|Default|GetCubeGridToolOutput_C6FC7464) (Math|Vector|Lerp(Vector) "-624.000000,123.375000,0.000000" "-624.000000,123.375000,250.000000" _newtrack_0) false false)
      (Transformation|SetRelativeLocation (Variables|Default|GetCubeGridToolOutput_A2B49A1B) (Math|Vector|Lerp(Vector) "0, 0, 0" "0.000000,0.000000,250.000000" _newtrack_0) false false))))

(fn ConstructionScript)