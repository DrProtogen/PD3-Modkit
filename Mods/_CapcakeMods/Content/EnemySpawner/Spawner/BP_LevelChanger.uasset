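; BP_LevelChanger switches levels through three custom events, covering a tutorial-based "PG" set and the ArmoredTransport map.
; LoadPG_Event and UnloadPG_Event stream the warehouse, combat architecture, props, lighting and PGUnits sublevels in or out, mostly with blocking calls.
; ArmouredTransport_Event opens ArmoredTransport as an absolute level change, then immediately spawns an SBZPlayerCharacter at the current player's transform.
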(event Custom|LoadPG_Event
  (Class|GameplayStatics|LoadStreamLevelbySoftObjectPtr "/Game/Prototype/Maps/Tutorial/Loud/LoudTutCombat/Sublevels/Environment_LoudTutCombat/E_LoudTutCombat_Arch.E_LoudTutCombat_Arch" true true)
  (Class|GameplayStatics|LoadStreamLevelbySoftObjectPtr "/Game/Prototype/Maps/Tutorial/Loud/LoudTutCombat/Sublevels/Environment_LoudTutCombat/E_LoudTutCombat_Prop.E_LoudTutCombat_Prop" true true)
  (Class|GameplayStatics|LoadStreamLevelbySoftObjectPtr "/Game/Prototype/Maps/Tutorial/_common/E_Tutorial_Warehouse.E_Tutorial_Warehouse" true true)
  (Class|GameplayStatics|LoadStreamLevelbySoftObjectPtr "/_CapcakeMods/EnemySpawner/Levels/PGUnits.PGUnits" true true)
  (Class|GameplayStatics|LoadStreamLevelbySoftObjectPtr "/Game/Prototype/Maps/Tutorial/Loud/LoudTutCombat/Sublevels/Lighting_LoudTutCombat/L_LoudTutCombat_Lighting.L_LoudTutCombat_Lighting" true false))

(event Custom|UnloadPG_Event
  (Class|GameplayStatics|UnloadStreamLevelbySoftObjectPtr "/Game/Prototype/Maps/Tutorial/_common/E_Tutorial_Warehouse.E_Tutorial_Warehouse" true)
  (Class|GameplayStatics|UnloadStreamLevelbySoftObjectPtr "/Game/Prototype/Maps/Tutorial/Loud/LoudTutCombat/Sublevels/Environment_LoudTutCombat/E_LoudTutCombat_Arch.E_LoudTutCombat_Arch" true)
  (Class|GameplayStatics|UnloadStreamLevelbySoftObjectPtr "/Game/Prototype/Maps/Tutorial/Loud/LoudTutCombat/Sublevels/Environment_LoudTutCombat/E_LoudTutCombat_Prop.E_LoudTutCombat_Prop" true)
  (Class|GameplayStatics|UnloadStreamLevelbySoftObjectPtr "/_CapcakeMods/EnemySpawner/Levels/PGUnits.PGUnits" false)
  (Class|GameplayStatics|UnloadStreamLevelbySoftObjectPtr "/Game/Prototype/Maps/Tutorial/Loud/LoudTutCombat/Sublevels/Lighting_LoudTutCombat/L_LoudTutCombat_Lighting.L_LoudTutCombat_Lighting" false))

(event Custom|ArmouredTransport_Event
  (bind _returnvalue (Game|GetPlayerCharacter 0))
  (Game|OpenLevel(byObjectReference) "/Game/Prototype/Maps/ArmoredTransport/ArmoredTransport.ArmoredTransport")
  (Game|SpawnActorfromClass "/Script/Starbreeze.SBZPlayerCharacter" (Transformation|GetActorTransform _returnvalue) "Undefined" "MultiplyWithRoot" _returnvalue _returnvalue))

(fn ConstructionScript)