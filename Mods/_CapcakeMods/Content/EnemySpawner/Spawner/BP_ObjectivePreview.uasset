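; BP_ObjectivePreview is an actor that displays an objective's name and variable states through a WBP_UI_ObjectivePreview widget component.
; The construction script passes the objective reference to the widget.
; Events forward the name with three variable values, hide all three variable rows, or update a variable's check state.
; The visibility event always sends Hidden, leaving its three visibility variables unused.
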(event Custom|Update%20Name_Event
  (bind _aswbp_ui_objective_preview (Utilities|Casting|CastToWBP_UI_ObjectivePreview (UserInterface|GetWidget (Variables|Default|GetWidget))))
  (Default|UpdateNameEvent _aswbp_ui_objective_preview (Utilities|Text|ToText(String) (Utilities|GetObjectName (Variables|Default|GetObjective%20Name))) (Variables|Default|Getvar1) (Variables|Default|Getvar2) (Variables|Default|Getvar3)))

(event Custom|Update%20Var%20Visibility_Event
  (bind _aswbp_ui_objective_preview (Utilities|Casting|CastToWBP_UI_ObjectivePreview (UserInterface|GetWidget (Variables|Default|GetWidget))))
  (Default|ToggleVariablesVisibilityEvent _aswbp_ui_objective_preview "Hidden" "Hidden" "Hidden"))

(event Custom|Update%20Var_Event
  (params (var :type objectivePreviewEnum%20Enum :default "NewEnumerator0") (Check%20State :type ECheckBoxState%20Enum :default "Unchecked"))
  (bind _aswbp_ui_objective_preview (Utilities|Casting|CastToWBP_UI_ObjectivePreview (UserInterface|GetWidget (Variables|Default|GetWidget))))
  (Default|UpdateVarChecksEvent _aswbp_ui_objective_preview var Check%20State))

(fn ConstructionScript
  (bind _aswbp_ui_objective_preview (Utilities|Casting|CastToWBP_UI_ObjectivePreview (UserInterface|GetWidget (Variables|Default|GetWidget))))
  (Variables|/_CapcakeMods/EnemySpawner/Spawner/WBP_UI_ObjectivePreview.WBP_UI_ObjectivePreview_C|SetbpRef _aswbp_ui_objective_preview (Variables|Default|GetObjective%20Name)))