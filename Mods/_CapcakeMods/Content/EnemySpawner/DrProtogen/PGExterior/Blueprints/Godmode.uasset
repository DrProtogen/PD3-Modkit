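; Godmode Blueprint that keeps a player's health and ammo topped up.
; Every Tick it looks up an SBZPlayerState with GetActorOfClass, so only the first one found is affected.
; It then calls multicast setters on that state's AttributeSet to force fixed values for health, weapon and throwable/placeable inventory ammo, and loaded magazines.
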(event EventBeginPlay
  (|CallParentFunction))

(event EventTick
  (params (DeltaSeconds :type Float%20%28single-precision%29))
  (Utilities|FlowControl|Sequence
    (:then_0
      (bind _returnvalue (Actor|GetActorOfClass "/Script/Starbreeze.SBZPlayerState"))
      (Utilities|FlowControl|Sequence
        (:then_0
          (Class|SBZPlayerAttributeSet|MulticastSetPrimaryEquippableAmmoInventory (Variables|/Script/Starbreeze.SBZPlayerState|GetAttributeSet _returnvalue) 1e+02))
        (:then_1
          (Class|SBZPlayerAttributeSet|MulticastSetSecondaryEquippableAmmoInventory (Variables|/Script/Starbreeze.SBZPlayerState|GetAttributeSet _returnvalue) 1e+02))
        (:then_2
          (Class|SBZPlayerAttributeSet|MulticastSetPrimaryPlaceableAmmoInventory (Variables|/Script/Starbreeze.SBZPlayerState|GetAttributeSet _returnvalue) 1e+02))
        (:then_3
          (Class|SBZPlayerAttributeSet|MulticastSetPrimaryThrowableAmmoInventory (Variables|/Script/Starbreeze.SBZPlayerState|GetAttributeSet _returnvalue) 1e+02))
        (:then_4
          (Class|SBZPlayerAttributeSet|MulticastSetPrimaryEquippableAmmoLoaded (Variables|/Script/Starbreeze.SBZPlayerState|GetAttributeSet _returnvalue) 32.0))
        (:then_5
          (Class|SBZPlayerAttributeSet|MulticastSetSecondaryEquippableAmmoLoaded (Variables|/Script/Starbreeze.SBZPlayerState|GetAttributeSet _returnvalue) 32.0))))
    (:then_1
      (bind _returnvalue_2 (Actor|GetActorOfClass "/Script/Starbreeze.SBZPlayerState"))
      (Class|SBZPawnAttributeSet|MulticastSetHealth (Variables|/Script/Starbreeze.SBZPlayerState|GetAttributeSet _returnvalue_2) 3e+02))))

(fn ConstructionScript
  (|CallParentFunction))