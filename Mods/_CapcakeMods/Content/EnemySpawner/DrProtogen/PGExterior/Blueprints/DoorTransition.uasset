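; Door transition actor that teleports the player when its grab handle interaction completes on the server.
; TeleportPlayer moves the local player pawn to the PawnSpawnUnit component's world location, raised slightly, and matches its rotation.
; A separate SpawnTeleportLocation event adds a static mesh component.
; Loading screen, delayed map load and spawn-array attachment logic are present but disconnected.
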(event OnServerCompleteInteraction(HandleGrab)
  (params (Interactable :type SBZ%20Base%20Interactable%20Component%20Object%20Reference) (Interactor :type SBZ%20Interactor%20Component%20Object%20Reference) (bIsLocallyControlledInteractor :type Boolean))
  (CallFunction|TeleportPlayer))

(event Custom|Spawn%20Teleport%20Location
  (AddComponent|AddStaticMeshComponent self false))

(event EventBeginPlay)

(fn ConstructionScript)

(fn TeleportPlayer
  (bind _pawnspawnunit (Variables|Default|GetPawnSpawnUnit))
  (bind _returnvalue (Transformation|GetWorldLocation _pawnspawnunit))
  (bind (_x _y _z) (Math|Vector|BreakVector _returnvalue))
  (Transformation|SetActorLocationAndRotation (Class|SBZPlayerLibrary|GetLocalPlayerPawn) (Math|Vector|MakeVector _x _y (+ _z 5e+01)) (Transformation|GetWorldRotation _pawnspawnunit) false true))