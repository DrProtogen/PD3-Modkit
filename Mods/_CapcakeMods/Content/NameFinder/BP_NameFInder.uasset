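; BP_NameFInder is a debug-style labeler that displays names and tags for pawn spawners at BeginPlay.
; It scans every actor for SBZPawnSpawnGroup or SBZPawnSpawnBase and creates text components joining a name with tags at indices 1–4.
; Group labels use the group's name but attach to the finder itself.
; Base labels attach to each spawner, but their name lookup omits the spawner.
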(event EventBeginPlay
  (bind _outactors (Actor|GetAllActorsOfClass "/Script/Engine.Actor"))
  (for _array_element _outactors
    (bind _assbzpawn_spawn_group (Utilities|Casting|CastToSBZPawnSpawnGroup _array_element)
      (:then
        (bind _returnvalue (AddComponent|AddTextRenderComponent false))
        (Rendering|Components|TextRender|SetText _returnvalue (Utilities|Text|ToText(String) (Utilities|String|Append (Utilities|GetObjectName _assbzpawn_spawn_group) " - " (Utilities|String|ToString(Name) (Utilities|Array|Get(acopy) (Variables|/Script/Engine.Actor|GetTags _assbzpawn_spawn_group) 1)) " - " (Utilities|String|ToString(Name) (Utilities|Array|Get(acopy) (Variables|/Script/Engine.Actor|GetTags _assbzpawn_spawn_group) 2)) " - " (Utilities|String|ToString(Name) (Utilities|Array|Get(acopy) (Variables|/Script/Engine.Actor|GetTags _assbzpawn_spawn_group) 3)) " - " (Utilities|String|ToString(Name) (Utilities|Array|Get(acopy) (Variables|/Script/Engine.Actor|GetTags _assbzpawn_spawn_group) 4))))))
      (:CastFailed
        (bind _assbzpawn_spawn_base (Utilities|Casting|CastToSBZPawnSpawnBase _array_element))
        (bind _returnvalue_2 (AddComponent|AddTextRenderComponent _assbzpawn_spawn_base false))
        (Rendering|Components|TextRender|SetText _returnvalue_2 (Utilities|Text|ToText(String) (Utilities|String|Append (Utilities|GetObjectName 0) " - " (Utilities|String|ToString(Name) (Utilities|Array|Get(acopy) (Variables|/Script/Engine.Actor|GetTags _assbzpawn_spawn_base) 1)) " - " (Utilities|String|ToString(Name) (Utilities|Array|Get(acopy) (Variables|/Script/Engine.Actor|GetTags _assbzpawn_spawn_base) 2)) " - " (Utilities|String|ToString(Name) (Utilities|Array|Get(acopy) (Variables|/Script/Engine.Actor|GetTags _assbzpawn_spawn_base) 3)) " - " (Utilities|String|ToString(Name) (Utilities|Array|Get(acopy) (Variables|/Script/Engine.Actor|GetTags _assbzpawn_spawn_base) 4)))))))))

(fn ConstructionScript
  (|CallParentFunction))